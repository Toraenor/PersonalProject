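; Enemy character for a free-flow combat system, handling player detection, counter animations and hit reactions.
; AI perception registers it with the player's AI Director and sets the blackboard target, undoing both after a short timer when sight or sensing fails.
; Damage plays gun or directional hit montages, skipped when the attacker is countering this enemy mid-counter montage.
; While targetable, a timer then resets enemy logic through its enemy component.
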(event OnTargetPerceptionUpdated(AIPerception)
  (params (Actor :type Actor%20Object%20Reference) (Stimulus :type AI%20Stimulus%20Structure))
  (bind _returnvalue (AI|GetBlackboard 0))
  (bind _returnvalue_2 (Actor|GetComponentbyClass Actor "/Game/FFCS/Blueprints/AC_AIDirector.AC_AIDirector_C"))
  ;[1 1 1] Comment
  (if (Variables|Default|GetTargetable)
    (if (== Actor (Game|GetPlayerCharacter 0))
      (if (.bSuccessfullySensed (Utilities|Struct|BreakAIStimulus Stimulus))
        (Development|PrintString (Utilities|String|Append (Utilities|String|MakeLiteralString "Sensed ") (Utilities|GetDisplayName Actor)))
        (Utilities|Time|ClearandInvalidateTimerbyHandle (Variables|Default|GetTargetCheckerTimerHandle))
        (Utilities|IsValid _returnvalue_2
          (:Is%20Valid
            (Default|AddEnemy _returnvalue_2 self))
          (:Is%20Not%20Valid
            _))
        (Utilities|IsValid _returnvalue
          (:Is%20Valid
            (AI|Components|Blackboard|SetValueasObject _returnvalue (Utilities|Name|MakeLiteralName "TargetActor") Actor)))
        (else
          (bind _returnvalue_3 (Utilities|Time|SetTimerbyEvent (delegate Custom|LostPlayer) 2.0))
          (Variables|Default|SetTargetCheckerTimerHandle _returnvalue_3))))))

(event Custom|ResetEnemyLogicToNormal
  (bind _ac_enemycomp (Variables|Default|GetAC_EnemyComp))
  ;[1 1 1] Comment
  (Utilities|IsValid _ac_enemycomp
    (:Is%20Valid
      (Default|ControlEnemyLogic _ac_enemycomp false)
      (Class|EnemyComponent|SetAttackPlayer (Variables|Default|GetAC_EnemyComp) false))))

(event Custom|LostPlayer
  (bind _returnvalue (Utilities|Name|MakeLiteralName "TargetActor"))
  (bind _returnvalue_2 (AI|GetBlackboard 0))
  (bind _returnvalue_3 (AI|GetBlackboard 0))
  (bind _returnvalue_4 (Utilities|Name|MakeLiteralName "TargetActor"))
  (bind _returnvalue_5 (AI|GetBlackboard 0))
  (bind _returnvalue_6 (AI|Components|Blackboard|GetValueasObject _returnvalue_3 _returnvalue_4))
  (bind _returnvalue_7 (AI|Components|Blackboard|GetValueasObject _returnvalue_5 _returnvalue))
  (bind _ascharacter (Utilities|Casting|CastToCharacter _returnvalue_6))
  (bind _returnvalue_8 (Actor|GetComponentbyClass _ascharacter "/Game/FFCS/Blueprints/AC_AIDirector.AC_AIDirector_C"))
  ;[1 1 1] Comment
  (Utilities|IsValid _returnvalue_5
    (:Is%20Valid
      (Utilities|IsValid _returnvalue_7
        (:Is%20Valid
          (Development|PrintString (Utilities|String|Append (Utilities|String|MakeLiteralString "Lost ") (Utilities|GetDisplayName _returnvalue_7)))
          (Utilities|IsValid _returnvalue_3
            (:Is%20Valid
              (Utilities|IsValid _returnvalue_6
                (:Is%20Valid
                  (Utilities|IsValid _returnvalue_8
                    (:Is%20Valid
                      (Default|RemoveEnemy _returnvalue_8 self))
                    (:Is%20Not%20Valid
                      _))
                  (Utilities|IsValid _returnvalue_2
                    (:Is%20Valid
                      (AI|Components|Blackboard|SetValueasObject _returnvalue_2 (Utilities|Name|MakeLiteralName "TargetActor") 0))))))))))))

(event Custom|PlayCounterAnim
  (params (StartPosition :type Float%20%28double-precision%29))
  (bind _mesh (Variables|Character|GetMesh))
  (bind _ac_enemycomp (Variables|Default|GetAC_EnemyComp))
  (bind _returnvalue (Components|SkeletalMesh|GetAnimInstance _mesh))
  (bind _aicountermontage (Variables|/Game/FFCS/Blueprints/AC_EnemyComp.AC_EnemyComp_C|GetAICounterMontage _ac_enemycomp))
  ;[1 1 1] Comment
  (Utilities|IsValid (Variables|Default|GetAC_EnemyComp)
    (:Is%20Valid
      (Utilities|IsValid _returnvalue
        (:Is%20Valid
          (Variables|Default|SetAnimInstance _returnvalue)
          (Animation|Montage|PlayMontage (Variables|Character|GetMesh) (Variables|/Game/FFCS/Blueprints/AC_EnemyComp.AC_EnemyComp_C|GetAICounterMontage (Variables|Default|GetAC_EnemyComp)) 1.0 StartPosition
            (:then
              (Class|AnimInstance|MontageSetNextSection (Variables|Default|GetAnimInstance) (Class|AnimMontage|GetSectionName _aicountermontage) (Class|AnimMontage|GetSectionName _aicountermontage 1) (Variables|/Game/FFCS/Blueprints/AC_EnemyComp.AC_EnemyComp_C|GetAICounterMontage (Variables|Default|GetAC_EnemyComp)))
              (Variables|/Game/FFCS/Blueprints/AC_EnemyComp.AC_EnemyComp_C|SetIsInCounterAnimPart (Variables|Default|GetAC_EnemyComp) true))
            (:OnCompleted
              (bind _ac_enemycomp_2 (Variables|Default|GetAC_EnemyComp :!label _label)
                (:then
                  (Default|FinishCounterAnimation _ac_enemycomp_2))
                (:else)))
            (:OnInterrupted
              (goto _label))))))))

(event EventBeginPlay
  (|CallParentFunction)
  (bind _output_get (Variables|Default|SetMaxHealth 3.0))
  (Variables|Default|SetCurrentHealth _output_get))

(event Game|Damage|EventAnyDamage
  (params (Damage :type Float%20%28single-precision%29) (DamageType :type Damage%20Type%20Object%20Reference) (InstigatedBy :type Controller%20Object%20Reference) (DamageCauser :type Actor%20Object%20Reference))
  (bind _returnvalue (Actor|GetComponentbyClass DamageCauser "/Game/FFCS/Blueprints/AC_FFCC.AC_FFCC_C"))
  (bind _returnvalue_2 (Class|FreeFlowCombatComponent|GetCounterEnemy _returnvalue))
  ;[1 1 1] Comment
  (Utilities|IsValid DamageCauser
    (:Is%20Valid
      (Utilities|IsValid _returnvalue
        (:Is%20Valid
          (Utilities|IsValid _returnvalue_2
            (:Is%20Valid
              (if (and (== _returnvalue_2 self) (Variables|/Game/FFCS/Blueprints/AC_EnemyComp.AC_EnemyComp_C|GetIsInCounterAnimPart (Variables|Default|GetAC_EnemyComp)))
                (Class|CharacterBase|ApplyDamages Damage "Fwd")
                (if (Variables|Default|GetTargetable) :!label _label
                  (Utilities|Time|SetTimerbyEvent (delegate Custom|ResetEnemyLogicToNormal) 1.0))
                (else
                  (bind (_hitanimation _hitdirection) (CallFunction|GetHitAnimation DamageCauser :!label _label_2))
                  (Animation|Montage|PlayMontage (Variables|Character|GetMesh) _hitanimation
                    (:then
                      (Class|CharacterBase|ApplyDamages Damage _hitdirection))
                    (:OnCompleted
                      (goto _label))
                    (:OnInterrupted
                      (goto _label))))))
            (:Is%20Not%20Valid
              (goto _label_2))))))))

(fn ConstructionScript
  (|CallParentFunction))

(fn GetHitAnimation
  (params (Instigator :type Actor%20Object%20Reference))
  (bind _ac_enemycomp (Variables|Default|GetAC_EnemyComp))
  (bind _returnvalue (Class|EnemyComponent|HitDirection _ac_enemycomp Instigator))
  (if (Utilities|Enum|Equal(Enum) (Variables|/Game/FFCS/Blueprints/AC_EnemyComp.AC_EnemyComp_C|GetAttackType _ac_enemycomp) "NewEnumerator1")
    (return "/Game/AnimStarterPack/AM_GunHit.AM_GunHit" _returnvalue)
    (else
      (return (Utilities|Select :Index _returnvalue :Fwd "/Game/FFCS/Animations/AnimMontages/Hit/AM_HitForward.AM_HitForward" :Right "/Game/FFCS/Animations/AnimMontages/Hit/AM_HitRight.AM_HitRight" :Backward "/Game/FFCS/Animations/AnimMontages/Hit/AM_HitBack.AM_HitBack" :Left "/Game/FFCS/Animations/AnimMontages/Hit/AM_HitLeft.AM_HitLeft") _returnvalue))))