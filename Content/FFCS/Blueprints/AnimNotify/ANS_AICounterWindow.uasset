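; Anim notify state that marks the window in an enemy animation during which AC_EnemyComp is flagged as counterable.
; On begin, unless the enemy is already in its counter anim part, it tints the owner's Niagara component light blue, restarts and shows it, and sets IsInCounterWindow.
; On end, it hides the effect and clears the flag, both only if a Niagara component exists.
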(fn ReceivedNotifyBegin
  (params (MeshComp :type Skeletal%20Mesh%20Component%20Object%20Reference) (Animation :type Anim%20Sequence%20Base%20Object%20Reference) (TotalDuration :type Float%20%28single-precision%29) (EventReference :type Anim%20Notify%20Event%20Reference%20Structure%20%28by%20ref%29))
  (bind _returnvalue (Components|GetOwner MeshComp))
  (bind _returnvalue_2 (Components|GetOwner MeshComp))
  (bind _returnvalue_3 (Actor|GetComponentbyClass _returnvalue "/Game/FFCS/Blueprints/AC_EnemyComp.AC_EnemyComp_C"))
  (bind _returnvalue_4 (Actor|GetComponentbyClass _returnvalue_2 "/Game/FFCS/Blueprints/AC_EnemyComp.AC_EnemyComp_C"))
  (bind _returnvalue_5 (Actor|GetComponentbyClass _returnvalue_2 "/Script/Niagara.NiagaraComponent"))
  (Utilities|IsValid _returnvalue_4
    (:Is%20Valid
      (if (not (Variables|/Game/FFCS/Blueprints/AC_EnemyComp.AC_EnemyComp_C|GetIsInCounterAnimPart _returnvalue_4))
        (Utilities|IsValid _returnvalue_5
          (:Is%20Valid
            (Niagara|SetNiagaraVariable(LinearColor) _returnvalue_5 "Color" (Math|Color|MakeColor 0.08091 0.727047 1.0))
            (Niagara|ReinitializeSystem _returnvalue_5)
            (Development|SetHiddeninGame _returnvalue_5 false false)
            (Utilities|IsValid _returnvalue_3
              (:Is%20Valid
                (Variables|/Game/FFCS/Blueprints/AC_EnemyComp.AC_EnemyComp_C|SetIsInCounterWindow _returnvalue_3 true)
                (return true)))))))))

(fn ReceivedNotifyEnd
  (params (MeshComp :type Skeletal%20Mesh%20Component%20Object%20Reference) (Animation :type Anim%20Sequence%20Base%20Object%20Reference) (EventReference :type Anim%20Notify%20Event%20Reference%20Structure%20%28by%20ref%29))
  (bind _returnvalue (Components|GetOwner MeshComp))
  (bind _returnvalue_2 (Actor|GetComponentbyClass _returnvalue "/Game/FFCS/Blueprints/AC_EnemyComp.AC_EnemyComp_C"))
  (bind _returnvalue_3 (Actor|GetComponentbyClass _returnvalue "/Script/Niagara.NiagaraComponent"))
  (Utilities|IsValid _returnvalue_3
    (:Is%20Valid
      (Development|SetHiddeninGame _returnvalue_3 true false)
      (Utilities|IsValid _returnvalue_2
        (:Is%20Valid
          (Variables|/Game/FFCS/Blueprints/AC_EnemyComp.AC_EnemyComp_C|SetIsInCounterWindow _returnvalue_2 false)
          (return true))))))