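; AI director component that coordinates a group of enemies fighting the player, keeping melee attacks to one at a time.
; AddEnemy registers targetable enemies, signals fight start, and launches two looping timers with randomized intervals.
; Attack checks pick a random non-gun enemy, avoiding the last attacker, when nobody is attacking.
; It also sends idle non-gun enemies to look for weapons and can toggle every enemy's logic.
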(event EventBeginPlay)

(event EventTick
  (params (DeltaSeconds :type Float%20%28single-precision%29)))

(fn AddEnemy
  (params (Enemy :type Actor%20Object%20Reference))
  (bind _asenemy_base (Utilities|Casting|CastToEnemyBase Enemy))
  (if (Variables|/Script/FFCS.EnemyBase|GetTargetable _asenemy_base)
    (bind _returnvalue (Utilities|Array|AddUnique (Variables|Default|GetEnemies) Enemy))
    (if (== 0 _returnvalue)
      (Default|CallEnterFight))
    (if (and (> (Utilities|Array|Length (Variables|Default|GetEnemies)) 0) (not (Utilities|Time|IsTimerActivebyHandle (Variables|Default|GetCheckAttackPlayerTH))))
      (bind _returnvalue_2 (Utilities|Time|SetTimerbyEvent (EventDispatchers|CreateEvent :!event CheckifPlayerUnderAttack) (Math|Random|RandomFloatinRange 0.25 0.75) true true))
      (Variables|Default|SetCheckAttackPlayerTH _returnvalue_2)
      (Utilities|Time|SetTimerbyEvent (EventDispatchers|CreateEvent :!event MakeEnemyGoforWeapon) (Math|Random|RandomFloatinRange 3.0 5.0) true true))))

(fn CheckifPlayerUnderAttack
  (LocalVariables|SetChooseAIToAttack true)
  (for _array_element (Variables|Default|GetEnemies)
    (Utilities|IsValid (Actor|GetComponentbyClass _array_element "/Game/FFCS/Blueprints/AC_EnemyComp.AC_EnemyComp_C")
      (:Is%20Valid
        (if (Default|GetAttackPlayer (Actor|GetComponentbyClass _array_element "/Game/FFCS/Blueprints/AC_EnemyComp.AC_EnemyComp_C"))
          (LocalVariables|SetChooseAIToAttack false)))))
  (if (LocalVariables|GetChooseAIToAttack)
    (bind _outitem (CallFunction|GetAnotherEnemytoAttack))
    (bind _canattack (CallFunction|CheckEnemyCanAttack _outitem))
    (if _canattack
      (Class|EnemyComponent|SetAttackPlayer (Actor|GetComponentbyClass _outitem "/Game/FFCS/Blueprints/AC_EnemyComp.AC_EnemyComp_C") true)
      (Variables|Default|SetLastEnemy _outitem))))

(fn RemoveEnemy
  (params (Enemy :type Actor%20Object%20Reference))
  (Utilities|Array|RemoveItem (Variables|Default|GetEnemies) Enemy)
  (if (<= (Utilities|Array|Length (Variables|Default|GetEnemies)) 0)
    (Utilities|Time|ClearandInvalidateTimerbyHandle (Variables|Default|GetCheckAttackPlayerTH))))

(fn ToggleAllEnemiesLogic
  (params (Disable :type Boolean))
  (for _array_element (Variables|Default|GetEnemies)
    (Default|ControlEnemyLogic (Actor|GetComponentbyClass _array_element "/Game/FFCS/Blueprints/AC_EnemyComp.AC_EnemyComp_C") Disable)))

(fn GetAnotherEnemytoAttack
  (bind _enemies (Variables|Default|GetEnemies))
  (bind _enemies_2 (Variables|Default|GetEnemies))
  (bind _output (Utilities|Array|Get(acopy) _enemies_2))
  (if (> (Utilities|Array|Length (Variables|Default|GetEnemies)) 1)
    (LocalVariables|SetEnemiesToPick _enemies)
    (for _array_element _enemies
      (if (CallFunction|DoesEnemyAttackwithGun _array_element)
        (Utilities|Array|RemoveItem (LocalVariables|GetEnemiesToPick) _array_element)))
    (Utilities|IsValid (Variables|Default|GetLastEnemy)
      (:Is%20Valid
        (if (Utilities|Array|ContainsItem (LocalVariables|GetEnemiesToPick) (Variables|Default|GetLastEnemy))
          (Utilities|Array|RemoveItem (LocalVariables|GetEnemiesToPick) (Variables|Default|GetLastEnemy))))
      (:Is%20Not%20Valid
        _))
    (return (.OutItem (Utilities|Array|Random (LocalVariables|GetEnemiesToPick))))
    (elif (and (Utilities|Array|IsNotEmpty (Variables|Default|GetEnemies)) (not (CallFunction|DoesEnemyAttackwithGun _output)))
      (return _output))))

(fn CheckEnemyCanAttack
  (params (Enemy :type Actor%20Object%20Reference))
  (bind _returnvalue (Actor|GetComponentbyClass Enemy "/Game/FFCS/Blueprints/AC_EnemyComp.AC_EnemyComp_C"))
  (Utilities|IsValid Enemy
    (:Is%20Valid
      (Utilities|IsValid _returnvalue
        (:Is%20Valid
          (if (Utilities|Enum|Equal(Enum) (Variables|/Game/FFCS/Blueprints/AC_EnemyComp.AC_EnemyComp_C|GetAttackType _returnvalue) "NewEnumerator0")
            (if (Variables|/Game/FFCS/Blueprints/AC_EnemyComp.AC_EnemyComp_C|GetLogicStopped _returnvalue)
              (return false)
              (else
                (return true)))
            (else
              (return false))))
        (:Is%20Not%20Valid
          (return false))))
    (:Is%20Not%20Valid
      (return false))))

(fn MakeEnemyGoforWeapon
  (bind _enemies (Variables|Default|GetEnemies))
  (LocalVariables|SetEnemiesToPick _enemies)
  (for _array_element _enemies
    (Utilities|IsValid (Actor|GetComponentbyClass _array_element "/Game/FFCS/Blueprints/AC_EnemyComp.AC_EnemyComp_C")
      (:Is%20Valid
        (if (Math|Boolean|ORBoolean (Variables|/Game/FFCS/Blueprints/AC_EnemyComp.AC_EnemyComp_C|GetAttackingPlayer (Actor|GetComponentbyClass _array_element "/Game/FFCS/Blueprints/AC_EnemyComp.AC_EnemyComp_C")) (Variables|/Game/FFCS/Blueprints/AC_EnemyComp.AC_EnemyComp_C|GetLogicStopped (Actor|GetComponentbyClass _array_element "/Game/FFCS/Blueprints/AC_EnemyComp.AC_EnemyComp_C")) (Utilities|Enum|Equal(Enum) (Variables|/Game/FFCS/Blueprints/AC_EnemyComp.AC_EnemyComp_C|GetAttackType (Actor|GetComponentbyClass _array_element "/Game/FFCS/Blueprints/AC_EnemyComp.AC_EnemyComp_C")) "NewEnumerator1"))
          (Utilities|Array|RemoveItem (LocalVariables|GetEnemiesToPick) _array_element)))))
  (Utilities|IsValid (.OutItem (Utilities|Array|Random (LocalVariables|GetEnemiesToPick)))
    (:Is%20Valid
      (Utilities|IsValid (Actor|GetComponentbyClass (.OutItem (Utilities|Array|Random (LocalVariables|GetEnemiesToPick))) "/Game/FFCS/Blueprints/AC_EnemyComp.AC_EnemyComp_C")
        (:Is%20Valid
          (Default|SetAIState (Actor|GetComponentbyClass (.OutItem (Utilities|Array|Random (LocalVariables|GetEnemiesToPick))) "/Game/FFCS/Blueprints/AC_EnemyComp.AC_EnemyComp_C") "LookForWeapons"))))))

(fn DoesEnemyAttackwithGun
  (params (Enemy :type Actor%20Object%20Reference))
  (bind _returnvalue (Actor|GetComponentbyClass Enemy "/Game/FFCS/Blueprints/AC_EnemyComp.AC_EnemyComp_C"))
  (Utilities|IsValid _returnvalue
    (:Is%20Valid
      (return (Utilities|Enum|Equal(Enum) (Variables|/Game/FFCS/Blueprints/AC_EnemyComp.AC_EnemyComp_C|GetAttackType _returnvalue) "NewEnumerator1")))
    (:Is%20Not%20Valid
      (return false))))